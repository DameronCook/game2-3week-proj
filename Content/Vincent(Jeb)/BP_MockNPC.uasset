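; Mock NPC that shows its line of dialogue on screen when its Talk event fires.
; Talk lazily creates a WBP_Dialogue widget for the first player controller, caches it in DialogueUI and adds it to the viewport.
; Each call then writes the Dialogue variable into the widget's DialogueText, reusing the widget while it remains valid.
; Nothing in this Blueprint triggers Talk or hides the widget.
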(event `/Game/Vincent(Jeb)/BPI_Dialogue.Talk`
  (`/Engine/EditorBlueprintResources/StandardMacros.IsValid` (`self.DialogueUI`)
    (:`Is Valid`
      _)
    (:`Is Not Valid`
      (bind _returnvalue (`|CreateWidget` "/Game/Vincent(Jeb)/WBP_Dialogue.WBP_Dialogue_C" (`GameplayStatics.GetPlayerController` 0)))
      (bind _output_get (set `self.DialogueUI` _returnvalue))
      (`UserWidget.AddToViewport` _output_get 0)))
  (`TextBlock.SetText` (`/Game/Vincent(Jeb)/WBP_Dialogue.DialogueText` (`self.DialogueUI`)) (`KismetTextLibrary.Conv_StringToText` (`self.Dialogue`))))

(fn `UserConstructionScript`)