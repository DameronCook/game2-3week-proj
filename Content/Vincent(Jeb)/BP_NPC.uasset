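; An NPC Blueprint that shows dialogue when interacted with and prints that it can talk when looked at.
; On BeginPlay it caches the player and loads its dialogue lines and billboard sprite from DT_NPC by NPCName.
; Each interaction reuses or creates a WBP_Dialogue widget and advances one line.
; After the last line, the next interaction removes the widget, resets the index and sets the player's CanMove to true.
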(event `self.ReceiveBeginPlay`
  (bind _asbp_dddplayer (cast `/Game/Caitlyn/Blueprints/Characters/BP_DDDPlayer` (`GameplayStatics.GetPlayerCharacter` 0)))
  (set `self.As BP DDDPlayer` _asbp_dddplayer)
  ; Retrieve NPC data for dialogue
  (bind _returnvalue (`|GetDataTableRow` "/Game/Vincent(Jeb)/DT_NPC.DT_NPC" (`self.NPC Name`))
    (:`then`
      (bind (_npcname _npcimage _npcdialogue) (break `/Game/Vincent(Jeb)/F_NPC` _returnvalue))
      (set `self.Dialogue Strings` _npcdialogue)
      (`BillboardComponent.SetSprite` (`self.Billboard`) _npcimage))))

(event `self.InteractWith`
  (bind _dialogueui (`self.DialogueUI`))
  ; Dialogue system
  (`/Engine/EditorBlueprintResources/StandardMacros.IsValid` _dialogueui
    (:`Is Valid`
      (if (not (`Widget.IsInViewport` _dialogueui))
        (`UserWidget.AddToViewport` (stale _output_get) 0 :!label _label)))
    (:`Is Not Valid`
      (bind _returnvalue (`|CreateWidget` "/Game/Vincent(Jeb)/WBP_Dialogue.WBP_Dialogue_C"))
      (bind _output_get (set `self.DialogueUI` _returnvalue))
      (goto _label)))
  (if (< (`self.TalkIndex`) (`KismetArrayLibrary.Array_Length` (`self.Dialogue Strings`)))
    (`TextBlock.SetText` (`/Game/Vincent(Jeb)/WBP_Dialogue.DialogueText` (`self.DialogueUI`)) (`KismetTextLibrary.Conv_StringToText` (`|GetArrayItem` (`self.Dialogue Strings`) (`self.TalkIndex`))))
    (`/Engine/EditorBlueprintResources/StandardMacros.IncrementInt` (`self.TalkIndex`))
    (else
      (`GameViewportSubsystem.RemoveWidget` (subsystem `GameViewportSubsystem`) (`self.DialogueUI`))
      (set `self.TalkIndex` 0)
      (set `/Game/Caitlyn/Blueprints/Characters/BP_DDDPlayer.CanMove` true (`self.As BP DDDPlayer`)))))

(event `self.LookAt`
  (`KismetSystemLibrary.PrintString` (`KismetStringLibrary.Concat_StrStr` (`KismetStringLibrary.Conv_NameToString` (`self.NPC Name`)) " can talk.")))

(fn `UserConstructionScript`)