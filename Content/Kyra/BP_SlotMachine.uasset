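; Slot machine actor that spins its three rollers automatically in an endless loop, starting shortly after BeginPlay.
; Each update of a timeline adds world roll to every roller, scaling the shared Roller1 track by a random multiple of 30 degrees re-rolled per update.
; When the timeline finishes, a short random delay precedes the next spin, with no input or result evaluation.
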(event `self.ReceiveBeginPlay`
  (`KismetSystemLibrary.Delay` 0.5)
  (`self.Spinny`))

(event `Spinny`
  (bind (_direction _roller1) (`Timeline|1x1` :!via `PlayFromStart`)
    (:`Update`
      (bind _returnvalue (* _roller1 (* (`KismetMathLibrary.RandomIntegerInRange` 1 6) 30)))
      (`SceneComponent.K2_AddWorldRotation` (`self.SM_SlotRoller`) (`KismetMathLibrary.MakeRotator` _returnvalue) false false)
      (`SceneComponent.K2_AddWorldRotation` (`self.SM_SlotRoller1`) (`KismetMathLibrary.MakeRotator` _returnvalue) false false)
      (`SceneComponent.K2_AddWorldRotation` (`self.SM_SlotRoller2`) (`KismetMathLibrary.MakeRotator` _returnvalue) false false))
    (:`Finished`
      (`KismetSystemLibrary.Delay` (`KismetMathLibrary.RandomFloatInRange` 0.6 1.5))
      (`self.Spinny`))))

(fn `UserConstructionScript`)