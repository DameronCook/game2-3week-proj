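; BP_DDDEnemy is an interactable overworld enemy that talks to the player, then starts a battle.
; On BeginPlay it loads its dialogue lines and billboard sprite from DT_Enemy by EnemyName.
; Each interaction advances WBP_Dialogue; once lines run out, it opens WBP_BattleHUD with UI-only input, passing itself and its row name so it can be deleted after battle.
; Looking at it prints a battle prompt.
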(event `self.ReceiveBeginPlay`
  ; Retrieve enemy data for display and dialogue
  (bind _returnvalue (`|GetDataTableRow` "/Game/Dameron/DT_Enemy.DT_Enemy" (`self.Enemy Name`))
    (:`then`
      (bind (_enemyname _enemylook _healthtotal _hitrange _hazardrange _dialoguestrings) (break `/Game/Dameron/F_Enemy` _returnvalue))
      (set `self.Dialogue Strings` _dialoguestrings)
      (`BillboardComponent.SetSprite` (`self.Billboard`) _enemylook))))

(event `/Game/Caitlyn/Blueprints/Characters/BPI_InteractInterface.InteractWith`
  ; Dialogue system
  (`/Engine/EditorBlueprintResources/StandardMacros.IsValid` (`self.DialogueUI`)
    (:`Is Valid`
      _)
    (:`Is Not Valid`
      (bind _returnvalue (`|CreateWidget` "/Game/Vincent(Jeb)/WBP_Dialogue.WBP_Dialogue_C"))
      (bind _output_get (set `self.DialogueUI` _returnvalue))
      (`UserWidget.AddToViewport` _output_get 0)))
  (if (< (`self.TalkIndex`) (`KismetArrayLibrary.Array_Length` (`self.Dialogue Strings`)))
    (`TextBlock.SetText` (`/Game/Vincent(Jeb)/WBP_Dialogue.DialogueText` (`self.DialogueUI`)) (`KismetTextLibrary.Conv_StringToText` (`|GetArrayItem` (`self.Dialogue Strings`) (`self.TalkIndex`))))
    (`/Engine/EditorBlueprintResources/StandardMacros.IncrementInt` (`self.TalkIndex`))
    (else
      (`GameViewportSubsystem.RemoveWidget` (subsystem `GameViewportSubsystem`) (`self.DialogueUI`))
      ; Display Battle HUD Widget and Disable Game Input
      (bind _returnvalue_2 (`|CreateWidget` "/Game/Dameron/WBP_BattleHUD.WBP_BattleHUD_C"))
      (bind _aswbp_battle_hud (cast `/Game/Dameron/WBP_BattleHUD` _returnvalue_2))
      (set `/Game/Dameron/WBP_BattleHUD.DDD_Enemy Ref` self _aswbp_battle_hud) ; Giving the HUD a reference to this specific enemy\nso we can delete it after battle
      (set `/Game/Dameron/WBP_BattleHUD.Enemy Row Name` (`self.Enemy Name`) _aswbp_battle_hud)
      (`UserWidget.AddToViewport` _returnvalue_2 0)
      (`WidgetBlueprintLibrary.SetInputMode_UIOnlyEx` (`GameplayStatics.GetPlayerController` 0) null))))

(event `/Game/Caitlyn/Blueprints/Characters/BPI_InteractInterface.LookAt`
  (`KismetSystemLibrary.PrintString` (`KismetStringLibrary.Concat_StrStr` (`KismetStringLibrary.Conv_NameToString` (`self.Enemy Name`)) ": Do you want to battle?")))

(fn `UserConstructionScript`)