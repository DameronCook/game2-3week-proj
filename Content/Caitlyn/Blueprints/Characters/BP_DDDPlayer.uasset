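; BP_DDDPlayer is a player character Blueprint that handles movement and interaction with nearby actors.
; Enhanced Input drives control-rotation-relative movement while CanMove is true and shifts a Box toward the last movement input.
; Box overlaps track one BPI_InteractInterface actor as CurrentlyLookingAt, notifying it on begin and rescanning remaining overlaps on end.
; Interacting sends that actor an interface message and disables movement, with no re-enable in this Blueprint.
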(event `EnhancedInput|/Game/Caitlyn/Input/Actions/IA_Move`
  (params (ActionValue :type "Vector2D Structure") (ElapsedSeconds :type "Float (double-precision)") (TriggeredSeconds :type "Float (double-precision)") (InputAction :type "InputAction Object Reference" :default "/Game/Caitlyn/Input/Actions/IA_Move.IA_Move"))
  (bind (_returnvalue_roll _returnvalue_pitch _returnvalue_yaw) (`KismetMathLibrary.BreakRotator` (`self.GetControlRotation`)))
  (bind (_returnvalue_roll_2 _returnvalue_pitch_2 _returnvalue_yaw_2) (`KismetMathLibrary.BreakRotator` (`self.GetControlRotation`)))
  ; Character Movement
  (:`Triggered`
    (if (`self.CanMove`)
      ;; Move Left/Right
      (`self.AddMovementInput` (`KismetMathLibrary.GetRightVector` (`KismetMathLibrary.MakeRotator` _returnvalue_roll 0.0 _returnvalue_yaw)) ActionValue_X)
      ;; Move Forward/Backward
      (`self.AddMovementInput` (`KismetMathLibrary.GetForwardVector` (`KismetMathLibrary.MakeRotator` 0.0 0.0 _returnvalue_yaw_2)) ActionValue_Y)
      ; Character Interaction
      ;; Adjust Box Location for Interaction
      (`SceneComponent.K2_SetRelativeLocation` (`self.Box`) (* (`self.GetLastMovementInputVector`) 50.0) false false))))

(event `self.Box.OnComponentBeginOverlap`
  (params (OverlappedComponent :type "PrimitiveComponent Object Reference") (OtherActor :type "Actor Object Reference") (OtherComp :type "PrimitiveComponent Object Reference") (OtherBodyIndex :type Integer) (bFromSweep :type Boolean) (SweepResult :type "HitResult Structure (by ref)"))
  ; Character Interaction
  ;; Set Currenly Looking At to Overlapped Actor
  (if (`KismetSystemLibrary.DoesImplementInterface` OtherActor "/Game/Caitlyn/Blueprints/Characters/BPI_InteractInterface.BPI_InteractInterface_C")
    (message `/Game/Caitlyn/Blueprints/Characters/BPI_InteractInterface.LookAt` OtherActor)
    (set `self.Currently Looking At` OtherActor)))

(event `self.Box.OnComponentEndOverlap`
  (params (OverlappedComponent :type "PrimitiveComponent Object Reference") (OtherActor :type "Actor Object Reference") (OtherComp :type "PrimitiveComponent Object Reference") (OtherBodyIndex :type Integer))
  ; Character Interaction
  ;; Reset or Return 1 Overlapped Actor
  (bind _actor (`self.Get Overlapping Interactives` OverlappedComponent))
  (set `self.Currently Looking At` _actor))

(event `EnhancedInput|/Game/Caitlyn/Input/Actions/IA_Interact`
  (params (ActionValue :type Boolean) (ElapsedSeconds :type "Float (double-precision)") (TriggeredSeconds :type "Float (double-precision)") (InputAction :type "InputAction Object Reference" :default "/Game/Caitlyn/Input/Actions/IA_Interact.IA_Interact"))
  ; Character Interaction
  ;; Interact with Overlapped Actor
  (:`Started`
    (bind _currently_looking_at (`self.Currently Looking At`)
      (:`then`
        (set `self.CanMove` false)
        (message `/Game/Caitlyn/Blueprints/Characters/BPI_InteractInterface.InteractWith` _currently_looking_at))
      (:`else`))))

(fn `Get Overlapping Interactives`
  (params (Box :type "PrimitiveComponent Object Reference"))
  (returns (Actor :type "Actor Object Reference") (Return :type Boolean))
  (for _array_element (`PrimitiveComponent.GetOverlappingActors` Box "/Script/Engine.Actor")
    (if (`KismetSystemLibrary.DoesImplementInterface` _array_element "/Game/Caitlyn/Blueprints/Characters/BPI_InteractInterface.BPI_InteractInterface_C")
      (return _array_element true)))
  (return null false))

(fn `UserConstructionScript`)